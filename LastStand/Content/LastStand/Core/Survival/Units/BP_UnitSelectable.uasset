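; BP_UnitSelectable is a clickable unit base for Last Stand that tells double clicks from simple clicks.
; ActorOnClicked feeds the DETECT_DOUBLECLICK macro, which uses a Gate held open by a short Delay to flag a second click.
; Simple click fires immediately on the first click, without waiting for the window to expire.
; Double click calls OnDoubleClicked, while simple click only prints a debug string.
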(event EventBeginPlay)

(event Collision|EventActorBeginOverlap
  (params (OtherActor :type Actor%20Object%20Reference)))

(event EventTick
  (params (DeltaSeconds :type Float%20%28single-precision%29)))

(event MouseInput|EventActorOnClicked
  (params (ButtonPressed :type Key%20Structure :default "None"))
  (Utilities|DETECTDOUBLECLICK
    (:DoubleClick
      (Development|PrintString "DoubleClick")
      (Class|UnitSelectable|OnDoubleClicked))
    (:SimpleClick
      (Development|PrintString "SimpleClick"))))

(event Input|ActionEvents|InputActionLeftMouseClick
  (params (Key :type Key%20Structure :default "None")))

(fn ConstructionScript)